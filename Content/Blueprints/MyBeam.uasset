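; MyBeam is an actor with a static mesh root whose material displays the beam's load as tension relative to resistance.
; On BeginPlay it creates a dynamic material instance from its Material and applies it to the root mesh.
; Every tick it sets that instance's Tension scalar parameter to Tension divided by Resistance, leaving the visual response to the material.
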(event `self.ReceiveBeginPlay`
  (`self.CreateMat`))

(event `self.ReceiveTick`
  (params (DeltaSeconds :type "Float (single-precision)"))
  (`self.UpdateMatColor`))

(fn `CreateMat`
  (bind _asstatic_mesh_component (cast `StaticMeshComponent` (`self.RootComponent`)))
  (bind _returnvalue (`KismetMaterialLibrary.CreateDynamicMaterialInstance` (`self.Material`)))
  (set `self.MatInstance` _returnvalue)
  (`PrimitiveComponent.SetMaterial` _asstatic_mesh_component 0 _returnvalue))

(fn `UpdateMatColor`
  (`MaterialInstanceDynamic.SetScalarParameterValue` (`self.MatInstance`) "Tension" (/ (`self.Tension`) (`self.Resistance`))))

(fn `UserConstructionScript`)